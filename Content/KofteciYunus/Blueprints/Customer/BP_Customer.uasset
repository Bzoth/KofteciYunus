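; BP_Customer is the customer Blueprint, showing an animated sprite-sheet face on a TV screen plane.
; Construction creates a dynamic instance of MI_TVFace, which the sprite update fills with texture, frame rate, width and start time from the DT_CustomerFaceData row for the current expression.
; Non-looping faces revert to Neutral after their duration, derived from 64-pixel frame width and FPS.
; Tick prints the material's scalar parameters for debugging.
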(event Custom|Sprite_Update
  (bind _face_dmi_ref (Variables|Default|GetFace_DMI_Ref))
  (Development|PrintString "Sprite Update!")
  (bind _returnvalue (Utilities|GetDataTableRow "/Game/KofteciYunus/Blueprints/Customer/DT_CustomerFaceData.DT_CustomerFaceData" (Utilities|Select :Index (Variables|Default|GetE_Customer_Faces) :NewEnumerator0 "Neutral" :NewEnumerator1 "Happy"))
    (:then
      (Rendering|Material|SetScalarParameterValue _face_dmi_ref "Time_offset" (Actor|GetGameTimeSinceCreation) :!class /Script/Engine.MaterialInstanceDynamic)
      (Rendering|Material|SetScalarParameterValue _face_dmi_ref "Anim_FPS" (.Anim_FPS (Utilities|Struct|BreakS_CustomerFaceData _returnvalue)) :!class /Script/Engine.MaterialInstanceDynamic)
      (Rendering|Material|SetTextureParameterValue _face_dmi_ref "Face_Texture" (.Face_Texture (Utilities|Struct|BreakS_CustomerFaceData _returnvalue)))
      (Rendering|Material|SetScalarParameterValue _face_dmi_ref "Sprite_Width" (Math|Conversions|ToFloat(Integer) (Class|Texture2D|BlueprintGetSizeX (.Face_Texture (Utilities|Struct|BreakS_CustomerFaceData _returnvalue)))) :!class /Script/Engine.MaterialInstanceDynamic)
      (if (not (.IsLooping? (Utilities|Struct|BreakS_CustomerFaceData _returnvalue)))
        (Utilities|FlowControl|Delay (/ (/ (Math|Conversions|ToFloat(Integer) (Class|Texture2D|BlueprintGetSizeX (.Face_Texture (Utilities|Struct|BreakS_CustomerFaceData _returnvalue)))) 64.0) (.Anim_FPS (Utilities|Struct|BreakS_CustomerFaceData _returnvalue))))
        (Variables|Default|SetE_Customer_Faces "NewEnumerator0")
        (CallFunction|SpriteUpdate)))
    (:RowNotFound
      (Development|PrintString "row not found"))))

(event EventBeginPlay
  (CallFunction|SpriteUpdate))

(event EventTick
  (params (DeltaSeconds :type Float%20%28single-precision%29))
  (for _array_element (Variables|/Script/Engine.MaterialInstance|GetScalarParameterValues (Variables|Default|GetFace_DMI_Ref))
    (Development|PrintString (Utilities|String|Append (Utilities|String|ToString(Name) (.name (.parameterinfo _array_element))) ": " (Utilities|String|ToString(Float) (.parametervalue _array_element))) true true "(R=0.000000,G=0.660000,B=1.000000,A=1.000000)" 0.0)))

(fn ConstructionScript
  (bind _returnvalue (Rendering|Material|CreateDynamicMaterialInstance "/Game/KofteciYunus/Assets/Materials/MaterialInstances/MI_TVFace.MI_TVFace" "None" "None" :!class /Script/Engine.KismetMaterialLibrary))
  (bind _output_get (Variables|Default|SetFace_DMI_Ref _returnvalue))
  (Rendering|Material|SetMaterial (Variables|Default|GetTV_Screen_plane) 0 _output_get)
  (Development|PrintString "Construction Run" true true "(R=1.000000,G=0.007144,B=0.000000,A=1.000000)"))