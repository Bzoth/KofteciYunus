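; BP_Knife is a hand-held kitchen tool whose Blade can be ignited and put out by input actions while it is held.
; GrabComponent events toggle player input and add or remove a left or right weapon Enhanced Input mapping context based on the holding hand.
; Igniting shows the Blade and plays a Timeline that drives its material color.
; Putting out hides it and stops the Timeline, while dropping also hides it.
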(event OnGrabbed(GrabComponent)
  (params (NewParam :type Motion%20Controller%20Component%20Object%20Reference))
  (Input|EnableInput (Game|GetPlayerController 0))
  (Input|AddMappingContext (PlayerController|LocalPlayerSubsystems|GetEnhancedInputLocalPlayerSubsystem (Game|GetPlayerController 0)) (select (Utilities|Enum|Equal(Enum) (Default|GetHeldbyHand (Variables|Default|GetGrabComponent)) "Right") "/Game/KofteciYunus/Input/IMC_Weapon_Right.IMC_Weapon_Right" "/Game/KofteciYunus/Input/IMC_Weapon_Left.IMC_Weapon_Left") 1 "(bIgnoreAllPressedKeysUntilRelease=True,bForceImmediately=False,bNotifyUserSettings=False)")
  (Default|CallGrabbed))

(event OnDropped(GrabComponent)
  (Input|DisableInput (Game|GetPlayerController 0))
  (Rendering|SetVisibility (Variables|Default|GetBlade) false false)
  (Input|RemoveMappingContext (PlayerController|LocalPlayerSubsystems|GetEnhancedInputLocalPlayerSubsystem (Game|GetPlayerController 0)) (select (Utilities|Enum|Equal(Enum) (Default|GetHeldbyHand (Variables|Default|GetGrabComponent)) "Right") "/Game/KofteciYunus/Input/IMC_Weapon_Right.IMC_Weapon_Right" "/Game/KofteciYunus/Input/IMC_Weapon_Left.IMC_Weapon_Left") "(bIgnoreAllPressedKeysUntilRelease=True,bForceImmediately=False,bNotifyUserSettings=False)"))

(event Input|EnhancedActionEvents|EnhancedInputActionIA_Ignite
  (params (ActionValue :type Boolean) (ElapsedSeconds :type Float%20%28double-precision%29) (TriggeredSeconds :type Float%20%28double-precision%29) (InputAction :type Input%20Action%20Object%20Reference :default "/Game/KofteciYunus/Input/Actions/IA_Ignite.IA_Ignite"))
  (:Started
    (Rendering|SetVisibility (Variables|Default|GetBlade) true false)
    (bind _newtrack_1 (Timeline|Timeline PlayFromStart)
      (:Update
        (Rendering|Material|SetColorParameterValueonMaterials (Variables|Default|GetBlade) "Color" (Utilities|Struct|MakeLinearColor (.r _newtrack_1) (.g _newtrack_1) (.b _newtrack_1) 1.0))))))

(event Input|EnhancedActionEvents|EnhancedInputActionIA_PutOut
  (params (ActionValue :type Boolean) (ElapsedSeconds :type Float%20%28double-precision%29) (TriggeredSeconds :type Float%20%28double-precision%29) (InputAction :type Input%20Action%20Object%20Reference :default "/Game/KofteciYunus/Input/Actions/IA_PutOut.IA_PutOut"))
  (Rendering|SetVisibility (Variables|Default|GetBlade) false false)
  (bind _newtrack_1 (Timeline|Timeline Stop)
    (:Update
      (Rendering|Material|SetColorParameterValueonMaterials (Variables|Default|GetBlade) "Color" (Utilities|Struct|MakeLinearColor (.r _newtrack_1) (.g _newtrack_1) (.b _newtrack_1) 1.0)))))

(fn ConstructionScript)