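; Kitchen drink dispenser barrel with a lever pulled by a motion controller.
; AddDrink destroys the passed cup and spawns a locked BP_BeerCup at the tap, whatever the drink type.
; While grabbed, a looping timer aims the clamped lever at the controller.
; On release, timers raise the lever; a full pull returns slower, filling the cup's material and DrinkAmount, and the cup becomes grabbable at the top.
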(event OnGrabbed(GrabComponent)
  (params (NewParam :type Motion%20Controller%20Component%20Object%20Reference))
  (Variables|Components|SetMotion%20Controller NewParam)
  (bind _returnvalue (Utilities|Time|SetTimerbyFunctionName 0 "LeverHoldTimerFunc" 0.01 true))
  (Variables|Default|SetLeverHoldRotationTimer _returnvalue))

(event OnDropped(GrabComponent)
  (Utilities|Time|ClearandInvalidateTimerbyHandle (Variables|Default|GetLeverHoldRotationTimer))
  (Variables|Components|SetMotion%20Controller 0)
  (CallFunction|LeverReleased))

(event EventAddDrink
  (params (Drink :type ST%20Drink%20Structure) (Cup :type BP%20Cup%20Object%20Reference))
  (bind _scene1 (Variables|Default|GetScene1))
  (bind _returnvalue (Transformation|GetWorldTransform _scene1))
  (Variables|Default|SetDrinkType (.drinktype Drink))
  (Utilities|IsValid Cup
    (:Is%20Valid
      (Actor|DestroyActor Cup))
    (:Is%20Not%20Valid
      _))
  (Variables|Default|SetDrinkValue 0.0)
  (bind _returnvalue_2 (Game|SpawnActorfromClass (Utilities|Select :Index (Variables|Default|GetDrinkType) :NewEnumerator0 "/Game/KofteciYunus/Blueprints/KitchenTools/BP_BeerCup.BP_BeerCup_C" :NewEnumerator1 "/Game/KofteciYunus/Blueprints/KitchenTools/BP_BeerCup.BP_BeerCup_C" :NewEnumerator2 "/Game/KofteciYunus/Blueprints/KitchenTools/BP_BeerCup.BP_BeerCup_C") (Math|Transform|MakeTransform (.location _returnvalue) (.rotation _returnvalue) "1.000000,1.000000,1.000000") "Undefined" "MultiplyWithRoot" 0 0))
  (bind _asbp_cup (Utilities|Casting|CastToBP_Cup _returnvalue_2))
  (Variables|Default|SetCurrentCup _asbp_cup)
  (Variables|/Game/KofteciYunus/Blueprints/Player/GrabComponent.GrabComponent_C|SetCanBeGrabbed (Variables|/Game/KofteciYunus/Blueprints/KitchenTools/BP_Cup.BP_Cup_C|GetGrabComponent _asbp_cup) false))

(fn ConstructionScript)

(fn LeverHoldTimerFunc
  (bind _motion_controller (Variables|Components|GetMotion%20Controller))
  (bind _leverbase (Variables|Components|GetLeverBase))
  (bind _returnvalue (Transformation|GetWorldLocation _leverbase))
  (bind _returnvalue_2 (Transformation|GetWorldLocation _motion_controller))
  (bind _returnvalue_3 (Math|Rotator|FindLookatRotation _returnvalue _returnvalue_2))
  (bind _returnvalue_4 (+ (.pitch _returnvalue_3) -85.0))
  (bind _returnvalue_5 (Math|Rotator|NormalizeAxis _returnvalue_4))
  (bind _returnvalue_6 (Math|Float|Clamp(Float) _returnvalue_5 -1.2e+02 -3e+01))
  (Variables|Default|SetLeverRotation _returnvalue_6)
  (Transformation|SetRelativeRotation (Variables|Components|GetLeverBase) (Math|Rotator|MakeRotator 0.0 _returnvalue_6 0.0) false false)
  (if (<= (Variables|Default|GetLeverRotation) -119.0)
    (Utilities|FlowControl|DoOnce false :!label _label
      (:Completed
        (Audio|SpawnSound2D "/Game/KofteciYunus/Assets/Audio/SW_LeverDown.SW_LeverDown" 1.0 1.0 0.0 0)
        (goto _label_2 Reset)))
    (elif (<= (Variables|Default|GetLeverRotation) -1.1e+02)
      (Utilities|FlowControl|DoOnce false :!label _label_2
        (:Completed
          (goto _label Reset))))))

(fn LeverReleased
  (Variables|/Game/KofteciYunus/Blueprints/Player/GrabComponent.GrabComponent_C|SetCanBeGrabbed (Variables|Components|GetGrabComponent) false)
  (bind _returnvalue (Utilities|Time|SetTimerbyFunctionName 0 (select (<= (Variables|Default|GetLeverRotation) -119.0) "FullLeverReleasedTimer" "LeverReleasedTimer") 0.01 true))
  (Variables|Default|SetLeverReleasedRotationTimer _returnvalue)
  (if (<= (Variables|Default|GetLeverRotation) -119.0)
    (Audio|SpawnSound2D "/Game/KofteciYunus/Assets/Audio/SW_FillDrink1.SW_FillDrink1" 0.5 1.0 0.3 0)))

(fn LeverReleasedTimer
  (bind _currentcup (Variables|Default|GetCurrentCup))
  (bind _output_get (Variables|Default|SetLeverRotation (+ (Variables|Default|GetLeverRotation) 1.0)))
  (Transformation|SetRelativeRotation (Variables|Components|GetLeverBase) (Math|Rotator|MakeRotator 0.0 _output_get 0.0) false false)
  (if (>= (Variables|Default|GetLeverRotation) -2e+01)
    (Utilities|Time|ClearandInvalidateTimerbyHandle (Variables|Default|GetLeverReleasedRotationTimer))
    (Audio|SpawnSound2D "/Game/KofteciYunus/Assets/Audio/SW_LeverUp.SW_LeverUp" 1.0 1.0 0.0 0)
    (Variables|/Game/KofteciYunus/Blueprints/Player/GrabComponent.GrabComponent_C|SetCanBeGrabbed (Variables|Components|GetGrabComponent) true)
    (Utilities|IsValid _currentcup
      (:Is%20Valid
        (Variables|/Game/KofteciYunus/Blueprints/Player/GrabComponent.GrabComponent_C|SetCanBeGrabbed (Variables|/Game/KofteciYunus/Blueprints/KitchenTools/BP_Cup.BP_Cup_C|GetGrabComponent _currentcup) true)))))

(fn FullLeverReleasedTimer
  (bind _currentcup (Variables|Default|GetCurrentCup))
  (bind _output_get (Variables|Default|SetLeverRotation (+ (Variables|Default|GetLeverRotation) 0.5)))
  (Transformation|SetRelativeRotation (Variables|Components|GetLeverBase) (Math|Rotator|MakeRotator 0.0 _output_get 0.0) false false)
  (Utilities|FlowControl|Sequence
    (:then_0
      (bind _currentcup_2 (Variables|Default|GetCurrentCup)
        (:then
          (Rendering|Material|SetScalarParameterValue (Variables|/Game/KofteciYunus/Blueprints/KitchenTools/BP_Cup.BP_Cup_C|GetLiquidMaterial _currentcup_2) "Fill_Amount" (Math|Float|Clamp(Float) (- 1.0 (/ (- -2e+01 (Variables|Default|GetLeverRotation)) 1e+02)) 0.0 0.7) :!class /Script/Engine.MaterialInstanceDynamic)
          (Variables|/Game/KofteciYunus/Blueprints/KitchenTools/BP_Cup.BP_Cup_C|SetDrinkAmount (Variables|Default|GetCurrentCup) (- 1.0 (/ (- -2e+01 (Variables|Default|GetLeverRotation)) 1e+02))))
        (:else)))
    (:then_1
      (if (>= (Variables|Default|GetLeverRotation) -2e+01)
        (Utilities|Time|ClearandInvalidateTimerbyHandle (Variables|Default|GetLeverReleasedRotationTimer))
        (Audio|SpawnSound2D "/Game/KofteciYunus/Assets/Audio/SW_LeverUp.SW_LeverUp" 1.0 1.0 0.0 0)
        (Variables|/Game/KofteciYunus/Blueprints/Player/GrabComponent.GrabComponent_C|SetCanBeGrabbed (Variables|Components|GetGrabComponent) true)
        (Utilities|IsValid _currentcup
          (:Is%20Valid
            (Variables|/Game/KofteciYunus/Blueprints/Player/GrabComponent.GrabComponent_C|SetCanBeGrabbed (Variables|/Game/KofteciYunus/Blueprints/KitchenTools/BP_Cup.BP_Cup_C|GetGrabComponent _currentcup) true)))))))

(fn AddBurgerIngredient
  (params (Base :type BP%20Bread%20Base%20Object%20Reference))
  (return "0, 0, 0" "NewEnumerator0" 0.0))