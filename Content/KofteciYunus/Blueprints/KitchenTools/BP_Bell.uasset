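; Kitchen bell actor paired with a Plate, which it signals by broadcasting BellRang when rung.
; Overlapping its trigger sphere plays the bell sound, then after a short delay either broadcasts and locks the bell or plays a fail sound.
; On BeginPlay it registers with the Plate and binds to its CanRing dispatcher to re-arm.
; An overlay material on the mesh marks when it can be pressed.
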(event OnComponentBeginOverlap(Sphere1)
  (params (OverlappedComponent :type Primitive%20Component%20Object%20Reference) (OtherActor :type Actor%20Object%20Reference) (OtherComp :type Primitive%20Component%20Object%20Reference) (OtherBodyIndex :type Integer) (bFromSweep :type Boolean) (SweepResult :type Hit%20Result%20Structure%20%28by%20ref%29))
  (Audio|SpawnSound2D "/Game/KofteciYunus/Assets/Audio/SW_Bell.SW_Bell" 1.0 1.0 0.0 0)
  (Utilities|FlowControl|Delay 1.0)
  (CallFunction|PressBell))

(event EventBeginPlay
  (bind _plate (Variables|Default|GetPlate))
  (EventDispatchers|AssignCanRing _plate (EventDispatchers|CreateEvent :!event CanRingAgain))
  (Variables|/Game/KofteciYunus/Blueprints/KitchenTools/BP_Plate.BP_Plate_C|SetBell _plate self))

(fn ConstructionScript)

(fn PressBell
  (if (Variables|Default|GetCanBePressed)
    (Default|CallBellRang self (Variables|Default|GetPlate))
    (Rendering|Material|SetOverlayMaterial (Variables|Default|GetSphere) 0 :!class /Script/Engine.MeshComponent)
    (Variables|Default|SetCanBePressed false)
    (else
      (Audio|SpawnSound2D "/Game/KofteciYunus/Assets/Audio/SW_BellFail.SW_BellFail" 1.0 1.0 0.0 0))))

(fn CanRingAgain
  (params (Bell :type BP%20Bell%20Object%20Reference) (Plate :type BP%20Plate%20Object%20Reference))
  (Variables|Default|SetCanBePressed true)
  (Rendering|Material|SetOverlayMaterial (Variables|Default|GetSphere) "/Game/KofteciYunus/Assets/BaseMaterial/M_BellOverlay.M_BellOverlay" :!class /Script/Engine.MeshComponent))