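; BP_CupSpawner is a kitchen tool actor that spawns BP_BeerCup actors at its own transform, starting with one on BeginPlay.
; SpawnCup unbinds from the previous cup's Grabbed event if that cup is still valid, then stores the new cup as LastCup.
; It binds to the new cup's Grabbed event, so only the most recently spawned cup stays hooked to the spawner.
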(event EventBeginPlay
  (CallFunction|SpawnCup))

(fn ConstructionScript)

(fn SpawnCup
  (bind _returnvalue (Game|SpawnActorfromClass "/Game/KofteciYunus/Blueprints/KitchenTools/BP_BeerCup.BP_BeerCup_C" (Transformation|GetActorTransform) "Undefined" "MultiplyWithRoot" 0 0))
  (Utilities|IsValid (Variables|Default|GetLastCup)
    (:Is%20Valid
      (EventDispatchers|UnbindEventfromGrabbed (Variables|Default|GetLastCup) (EventDispatchers|CreateEvent :!event SpawnCup)))
    (:Is%20Not%20Valid
      _))
  (bind _output_get (Variables|Default|SetLastCup _returnvalue))
  (EventDispatchers|BindEventtoGrabbed _output_get (EventDispatchers|CreateEvent :!event SpawnCup)))