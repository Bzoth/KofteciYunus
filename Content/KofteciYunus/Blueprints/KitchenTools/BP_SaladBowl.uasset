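; Salad bowl kitchen tool that collects lettuce and tomato and can be chopped with a knife.
; Added ingredients and knife overlaps step each vegetable through state-indexed mesh maps; added ingredient actors are destroyed and recorded with state and mesh.
; Chop progress, or a finished state on adding, makes the bowl grabbable.
; On drop, it re-enables physics, sphere-traces at itself and messages the salad data to the hit actor for plating.
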(event OnDropped(GrabComponent)
  (bind _bowlmesh (Variables|Default|GetBowlMesh))
  (bind _returnvalue (Transformation|GetWorldLocation _bowlmesh))
  (Physics|SetSimulatePhysics (Variables|Default|GetBowlMesh) true)
  (bind _outhit (Collision|SphereTraceByChannel _returnvalue _returnvalue 1e+01 "TraceTypeQuery1" false 0 "None"))
  (Class|BPIInterract|SendSaladtoPlate(Message) (.HitActor (Collision|BreakHitResult _outhit)) (Variables|Default|GetSaladIngredients) (Variables|Default|GetSaladMeshes) self))

(event OnComponentBeginOverlap(BowlMesh)
  (params (OverlappedComponent :type Primitive%20Component%20Object%20Reference) (OtherActor :type Actor%20Object%20Reference) (OtherComp :type Primitive%20Component%20Object%20Reference) (OtherBodyIndex :type Integer) (bFromSweep :type Boolean) (SweepResult :type Hit%20Result%20Structure%20%28by%20ref%29))
  (if (Actor|ActorHasTag OtherActor "Knife")
    (CallFunction|SaladIngedient "NewEnumerator3")))

(event OnComponentEndOverlap(Box)
  (params (OverlappedComponent :type Primitive%20Component%20Object%20Reference) (OtherActor :type Actor%20Object%20Reference) (OtherComp :type Primitive%20Component%20Object%20Reference) (OtherBodyIndex :type Integer))
  (if (Actor|ActorHasTag OtherActor "Knife")
    (Variables|Default|SetCanBeChopped true)))

(event OnGrabbed(GrabComponent)
  (params (NewParam :type Motion%20Controller%20Component%20Object%20Reference))
  (Physics|SetSimulatePhysics (Variables|Default|GetBowlMesh) false))

(event EventAddSaladIngredient
  (params (Ingredient :type E_Salad%20Enum :default "NewEnumerator0") (Igredient :type BP%20Ingredient%20Object%20Reference))
  (CallFunction|SaladIngedient Ingredient Igredient))

(fn ConstructionScript)

(fn SaladIngedient
  (params (IngredientType :type E_Salad%20Enum :default "NewEnumerator0") (Ingredient :type BP%20Ingredient%20Object%20Reference))
  (switch Utilities|FlowControl|Switch|SwitchonE_Salad IngredientType
    (:NewEnumerator0
      (if (Variables|Default|GetLettuce)
        _
        (else
          (Rendering|SetVisibility (Variables|Default|GetSM_Lettuce) true false)
          (Variables|Default|SetLettuce true)))
      (if (<= (Variables|Default|GetLettuceState) 4)
        (CallFunction|ProgressLettuce Ingredient)))
    (:NewEnumerator1
      (if (Variables|Default|GetTomato)
        _
        (else
          (Rendering|SetVisibility (Variables|Default|GetSM_Tomato) true false)
          (Variables|Default|SetTomato true)))
      (if (<= (Variables|Default|GetTomatoState) 4)
        (CallFunction|ProgressTomato Ingredient)))
    (:NewEnumerator3
      (if (Variables|Default|GetCanBeChopped)
        (Utilities|FlowControl|Sequence
          (:then_0
            (if (Variables|Default|GetTomato)
              (if (<= (Variables|Default|GetTomatoState) 4)
                (CallFunction|ProgressTomato Ingredient)
                (Variables|Default|SetCanBeChopped true)
                (Variables|/Game/KofteciYunus/Blueprints/Player/GrabComponent.GrabComponent_C|SetCanBeGrabbed (Variables|Default|GetGrabComponent) true))))
          (:then_1
            (if (Variables|Default|GetLettuce)
              (if (<= (Variables|Default|GetLettuceState) 4)
                (CallFunction|ProgressLettuce Ingredient)
                (Variables|Default|SetCanBeChopped true)
                (Variables|/Game/KofteciYunus/Blueprints/Player/GrabComponent.GrabComponent_C|SetCanBeGrabbed (Variables|Default|GetGrabComponent) true)))))))))

(fn ProgressLettuce
  (params (Ingredients :type Actor%20Object%20Reference))
  (Math|Integer|IncrementInt (Variables|Default|GetLettuceState)
    (:%20%20
      (Components|StaticMesh|SetStaticMesh (Variables|Default|GetSM_Lettuce) (.Value (Utilities|Map|Find (Variables|Default|GetLettuceToMesh) (Variables|Default|GetLettuceState))))
      (Utilities|IsValid Ingredients
        (:Is%20Valid
          (Actor|DestroyActor Ingredients)
          (Utilities|Map|Add (Variables|Default|GetSaladIngredients) "NewEnumerator0" (Variables|Default|GetLettuceState))
          (Utilities|Map|Add (Variables|Default|GetSaladMeshes) "NewEnumerator0" (Variables|/Script/Engine.StaticMeshComponent|GetStaticMesh (Variables|Default|GetSM_Lettuce)))
          (if (> (Variables|Default|GetLettuceState) 4)
            (Variables|/Game/KofteciYunus/Blueprints/Player/GrabComponent.GrabComponent_C|SetCanBeGrabbed (Variables|Default|GetGrabComponent) true)))))))

(fn ProgressTomato
  (params (Ingredient :type Actor%20Object%20Reference))
  (Math|Integer|IncrementInt (Variables|Default|GetTomatoState)
    (:%20%20
      (Components|StaticMesh|SetStaticMesh (Variables|Default|GetSM_Tomato) (.Value (Utilities|Map|Find (Variables|Default|GetTomatoToMesh) (Variables|Default|GetTomatoState))))
      (Utilities|IsValid Ingredient
        (:Is%20Valid
          (Actor|DestroyActor Ingredient)
          (Utilities|Map|Add (Variables|Default|GetSaladIngredients) "NewEnumerator1" (Variables|Default|GetTomatoState))
          (Utilities|Map|Add (Variables|Default|GetSaladMeshes) "NewEnumerator1" (Variables|/Script/Engine.StaticMeshComponent|GetStaticMesh (Variables|Default|GetSM_Tomato)))
          (if (> (Variables|Default|GetTomatoState) 4)
            (Variables|/Game/KofteciYunus/Blueprints/Player/GrabComponent.GrabComponent_C|SetCanBeGrabbed (Variables|Default|GetGrabComponent) true)))))))

(fn AddBurgerIngredient
  (params (Base :type BP%20Bread%20Base%20Object%20Reference))
  (return "0, 0, 0" "NewEnumerator0" 0.0))