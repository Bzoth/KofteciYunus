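; BP_Cup is a grabbable physics cup that carries a drink type and amount for placement in cup holders.
; Grabbing turns physics off and dropping turns it back on, with CallGrabbed fired only on the first drop.
; A drop with DrinkAmount below 1 sphere-traces for CupHolder-tagged components and sends their actors an AddDrink message with the cup and drink data.
; BeginPlay stores a dynamic material as LiquidMaterial.
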(event OnDropped(GrabComponent)
  (bind _staticmesh (Variables|Default|GetStaticMesh))
  (bind _returnvalue (Transformation|GetWorldLocation _staticmesh))
  (Utilities|FlowControl|Sequence
    (:then_0
      (Utilities|FlowControl|DoOnce false
        (:Completed
          (Default|CallGrabbed))))
    (:then_1
      (Physics|SetSimulatePhysics (Variables|Default|GetStaticMesh) true))
    (:then_2
      (if (< (Variables|Default|GetDrinkAmount) 1.0)
        (bind _outhits (Collision|MultiSphereTraceByChannel _returnvalue _returnvalue 2e+01 "TraceTypeQuery1" false 0 "None"))
        (for _array_element _outhits
          (Utilities|IsValid (.HitActor (Collision|BreakHitResult _array_element))
            (:Is%20Valid
              (if (Components|ComponentHasTag (.HitComponent (Collision|BreakHitResult _array_element)) "CupHolder")
                (Class|BPIInterract|AddDrink(Message) (.HitActor (Collision|BreakHitResult _array_element)) (Utilities|Struct|MakeST_Drink (Variables|Default|GetDrinkType) (Variables|Default|GetDrinkAmount)) self)))))))))

(event OnGrabbed(GrabComponent)
  (params (NewParam :type Motion%20Controller%20Component%20Object%20Reference))
  (Physics|SetSimulatePhysics (Variables|Default|GetStaticMesh) false))

(event EventBeginPlay
  (bind _returnvalue (Rendering|Material|CreateDynamicMaterialInstance (Variables|Default|GetStaticMesh) 0 (Rendering|Material|GetMaterial (Variables|Default|GetStaticMesh) 0) "None" :!class /Script/Engine.PrimitiveComponent))
  (Variables|Default|SetLiquidMaterial _returnvalue))

(fn ConstructionScript)