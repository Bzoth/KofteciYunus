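; BP_Grill is a kitchen tool that cooks meatballs placed on it.
; When a BP_Meatball overlaps its Box, the grill releases it from any grab through its GrabComponent and sends it a start-cooking message.
; Leaving the Box sends a stop-cooking message, so the grill only signals the meatball and holds no cooking logic itself.
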(event OnComponentBeginOverlap(Box)
  (params (OverlappedComponent :type Primitive%20Component%20Object%20Reference) (OtherActor :type Actor%20Object%20Reference) (OtherComp :type Primitive%20Component%20Object%20Reference) (OtherBodyIndex :type Integer) (bFromSweep :type Boolean) (SweepResult :type Hit%20Result%20Structure%20%28by%20ref%29))
  (if (Utilities|ClassIsChildOf (Utilities|GetClass OtherActor) "/Game/KofteciYunus/Blueprints/Ingredients/BP_Meatball.BP_Meatball_C")
    (Default|TryRelease (Actor|GetComponentbyClass OtherActor "/Game/KofteciYunus/Blueprints/Player/GrabComponent.GrabComponent_C"))
    (Class|BPIInterract|StartCooking(Message) OtherActor)))

(event OnComponentEndOverlap(Box)
  (params (OverlappedComponent :type Primitive%20Component%20Object%20Reference) (OtherActor :type Actor%20Object%20Reference) (OtherComp :type Primitive%20Component%20Object%20Reference) (OtherBodyIndex :type Integer))
  (if (Utilities|ClassIsChildOf (Utilities|GetClass OtherActor) "/Game/KofteciYunus/Blueprints/Ingredients/BP_Meatball.BP_Meatball_C")
    (Class|BPIInterract|StopCooking(Message) OtherActor)))

(fn ConstructionScript)