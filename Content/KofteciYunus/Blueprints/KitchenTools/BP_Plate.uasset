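; Kitchen plate that receives a finished burger and rebuilds it as stacked static meshes on the plate.
; SendtoPlate runs once until ResetPlate, shows the bottom bun, calls CreateBurger and destroys the incoming burger actor.
; CreateBurger raises an Ingredient marker by per-type offsets, spawning randomly yawed meshes and setting each patty's doneness through a dynamic material Cook_Factor.
; ClearPlateItems empties the stored data, destroys the meshes and hides the bun.
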(event Custom|ResetPlate
  (Utilities|FlowControl|DoOnce false) ; enters at Reset
)

(event EventSendtoPlate
  (params (Ingredients :type Array%20of%20E_Ingredient%20Enums :default "NewEnumerator0") (PattyDegrees :type Array%20of%20Floats%20%28double-precision%29) (Burger :type Actor%20Object%20Reference))
  (Utilities|FlowControl|DoOnce false
    (:Completed
      (Rendering|SetVisibility (Variables|Default|GetBottomBun) true false)
      (CallFunction|CreateBurger Ingredients PattyDegrees)
      (Actor|DestroyActor Burger))))

(fn ConstructionScript)

(fn CreateBurger
  (params (Ingredients :type Array%20of%20E_Ingredient%20Enums :default "NewEnumerator0") (PattyDegrees :type Array%20of%20Floats%20%28double-precision%29))
  (bind _output_get (Variables|Default|SetIngredients Ingredients))
  (Variables|Default|SetPatty%20Degrees PattyDegrees)
  (Variables|Default|SetPattyAmount 0)
  (for _array_element _output_get
    (Transformation|AddLocalOffset (Variables|Default|GetIngredient) (.Offset (CallFunction|EnumtoMeshandOffset _array_element)) false false)
    (bind _returnvalue (AddComponent|AddStaticMeshComponent false (Math|Transform|MakeTransform "0, 0, 0" (Math|Rotator|MakeRotator 0.0 0.0 (Math|Random|RandomFloatinRange 0.0 3.6e+02)) "1.000000,1.000000,1.000000")))
    (Utilities|Array|Add (Variables|Default|GetIngredientMeshes) _returnvalue)
    (Transformation|AttachComponentToComponent _returnvalue (Variables|Default|GetBurger) "None" "KeepRelative" "KeepRelative" "KeepRelative" true)
    (Collision|SetCollisionEnabled _returnvalue "QueryOnly")
    (Transformation|SetRelativeLocation _returnvalue (Variables|/Script/Engine.SceneComponent|GetRelativeLocation (Variables|Default|GetIngredient)) false false)
    (Components|StaticMesh|SetStaticMesh _returnvalue (.Mesh (CallFunction|EnumtoMeshandOffset _array_element)))
    (if (Utilities|Enum|Equal(Enum) _array_element "NewEnumerator0")
      (bind _returnvalue_2 (Rendering|Material|CreateDynamicMaterialInstance _returnvalue 0 (Rendering|Material|GetMaterial _returnvalue 0) "None" :!class /Script/Engine.PrimitiveComponent))
      (bind _result (Math|Integer|IncrementInt (Variables|Default|GetPattyAmount))
        (:%20%20
          (Rendering|Material|SetScalarParameterValue _returnvalue_2 "Cook_Factor" (Utilities|Array|Get(acopy) (Variables|Default|GetPatty%20Degrees) (- _result 1)) :!class /Script/Engine.MaterialInstanceDynamic))))))

(fn EnumtoMeshandOffset
  (params (Ingredient :type E_Ingredient%20Enum :default "NewEnumerator0"))
  (return (Utilities|Select :Index Ingredient :NewEnumerator0 "/Game/KofteciYunus/Assets/StaticMeshes/SM_Patty.SM_Patty" :NewEnumerator1 "/Game/KofteciYunus/Assets/StaticMeshes/SM_Lettuce.SM_Lettuce" :NewEnumerator2 "/Game/KofteciYunus/Assets/StaticMeshes/SM_TomatoSlice.SM_TomatoSlice" :NewEnumerator3 "/Game/KofteciYunus/Assets/StaticMeshes/SM_Cheese.SM_Cheese" :NewEnumerator4 "/Game/KofteciYunus/Assets/StaticMeshes/SM_TopBun.SM_TopBun" :NewEnumerator5 0) (Utilities|Select :Index Ingredient :NewEnumerator0 "0.000000,0.000000,4.000000" :NewEnumerator1 "0.000000,0.000000,1.000000" :NewEnumerator2 "0.000000,0.000000,2.000000" :NewEnumerator3 "0.000000,0.000000,1.000000" :NewEnumerator4 "0.000000,0.000000,2.000000" :NewEnumerator5 "0, 0, 0")))

(fn ClearPlateItems
  (Utilities|Array|Clear (Variables|Default|GetIngredients))
  (Utilities|Array|Clear (Variables|Default|GetPatty%20Degrees))
  (Variables|Default|SetPattyAmount 0)
  (for _array_element (Variables|Default|GetIngredientMeshes)
    (Components|DestroyComponent _array_element))
  (Rendering|SetVisibility (Variables|Default|GetBottomBun) false false))

(fn Offset
  (params (Base :type BP%20Bread%20Base%20Object%20Reference))
  (return "0, 0, 0" "NewEnumerator0" 0.0))