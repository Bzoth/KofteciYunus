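; BP_Lever is a grabbable kitchen-tool lever that pivots to follow the hand holding it.
; On grab it stores the motion controller and starts a fast looping timer; on drop it clears both.
; Each tick, RotatorFunc aims the Scene pivot at the controller using look-at pitch with an offset, clamped to a fixed range, so the lever swings on one axis only.
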(event OnGrabbed(GrabComponent)
  (params (NewParam :type Motion%20Controller%20Component%20Object%20Reference))
  (Variables|Components|SetMotion%20Controller NewParam)
  (bind _returnvalue (Utilities|Time|SetTimerbyFunctionName 0 "RotatorFunc" 0.01 true))
  (Variables|Default|SetRotationTimer _returnvalue))

(event OnDropped(GrabComponent)
  (Utilities|Time|ClearandInvalidateTimerbyHandle (Variables|Default|GetRotationTimer))
  (Variables|Components|SetMotion%20Controller 0))

(fn ConstructionScript)

(fn RotatorFunc
  (Transformation|SetRelativeRotation (Variables|Components|GetScene) (Math|Rotator|MakeRotator 0.0 (Math|Float|Clamp(Float) (Math|Rotator|NormalizeAxis (+ (.pitch (Math|Rotator|FindLookatRotation (Transformation|GetWorldLocation (Variables|Components|GetScene)) (Transformation|GetWorldLocation (Variables|Components|GetMotion%20Controller)))) -85.0)) -1.2e+02 -3e+01) 0.0) false false))