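; BP_OrderManager runs the order loop of a burger-serving game, spawning customers and scoring served plates.
; A looping timer claims the first free row spline and spawns a customer there with its paired bell and a randomized burger, drink and salad order.
; Bell rings trigger payment from burger accuracy, drink match and salad ingredient-count difference.
; It then clears the plate, re-arms the bell and broadcasts the payment through it.
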(event EventBeginPlay
  (bind _outactors (Actor|GetAllActorsOfClass "/Game/KofteciYunus/Blueprints/KitchenTools/BP_Bell.BP_Bell_C"))
  (for _array_element _outactors
    (EventDispatchers|BindEventtoBellRang _array_element (EventDispatchers|CreateEvent :!event BellRang)))
  (Utilities|Time|SetTimerbyFunctionName 0 "NewCustomer" 5.0 true))

(fn ConstructionScript)

(fn BellRang
  (params (Bell :type BP%20Bell%20Object%20Reference) (Plate :type BP%20Plate%20Object%20Reference))
  (bind _order (Variables|/Game/KofteciYunus/Blueprints/KitchenTools/BP_Plate.BP_Plate_C|GetOrder Plate))
  (bind (_ingredients _pattydegrees) (Utilities|Struct|BreakST_Burger (.burger _order)))
  (Variables|Default|SetOrderCost 1e+02)
  (bind _totalaccuracy (Default|CalculateFinalBurgerAccuracy Plate _ingredients _pattydegrees))
  (bind _output_get (Variables|Default|SetOrderCost (+ (* _totalaccuracy (Variables|Default|GetOrderCost)) (select (== (.drink _order) (Variables|/Game/KofteciYunus/Blueprints/KitchenTools/BP_Plate.BP_Plate_C|GetHasDrink Plate)) 25.0 0.0) (Utilities|Select :Index (Math|Integer|Absolute(Integer) (- (Utilities|Array|Length (Utilities|Struct|BreakST_Salad (.salad _order))) (Utilities|Array|Length (.saladingredient (Variables|/Game/KofteciYunus/Blueprints/KitchenTools/BP_Plate.BP_Plate_C|GetSaladIngredients Plate))))) :Option%200 25.0 :Option%201 12.0 :Option%202 0.0))))
  (Development|PrintString (Utilities|String|Append "Final payment: " (Utilities|String|ToString(Float) _output_get)) true true "(R=0.000000,G=1.000000,B=0.398209,A=1.000000)" 3e+01)
  (Default|ClearPlateItems Plate)
  (Default|CanRingAgain Bell Bell Plate)
  (Default|CallOrderServed Bell (Variables|Default|GetOrderCost)))

(fn NewCustomer
  (bind _possibleorders (Variables|Default|GetPossibleOrders))
  (bind _outitem (Utilities|Array|Random _possibleorders))
  (bind (_1 _2 _3 _4) (Utilities|Struct|BreakST_RandomOrder _outitem))
  (bind (_array_element _array_index) (Utilities|Array|ForEachLoopwithBreak (Variables|Default|GetRows) :!label _label)
    (:LoopBody
      (if (not (Variables|/Game/KofteciYunus/Blueprints/Customer/BP_CustomerSpline.BP_CustomerSpline_C|GetOccupiced _array_element))
        (Variables|/Game/KofteciYunus/Blueprints/Customer/BP_CustomerSpline.BP_CustomerSpline_C|SetOccupiced _array_element true)
        (Utilities|FlowControl|Sequence
          (:then_0
            (goto _label Break))
          (:then_1
            (Game|SpawnActorfromClass "/Game/KofteciYunus/Blueprints/Customer/BP_Customer.BP_Customer_C" (Math|Transform|MakeTransform "0, 0, 0" "0, 0, 0" "1.000000,1.000000,1.000000") "Undefined" "MultiplyWithRoot" 0 _array_element (Utilities|Array|Get(acopy) (Variables|Default|GetBells) _array_index) (Utilities|Struct|MakeST_Order (Utilities|Struct|MakeST_Burger (Utilities|Array|MakeArray _1 _2 _3 _4) 1.0) (Math|Random|RandomBool) (Utilities|Struct|MakeST_Salad (select (Math|Random|RandomBool) "NewEnumerator0" (Utilities|Array|MakeArray "NewEnumerator1" "NewEnumerator0")))) 0)))))))