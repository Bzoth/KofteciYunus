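; Bottom bun of a burger that builds a stack from ingredients that hit it and hands it to a plate when dropped.
; Each accepted ingredient is destroyed and replaced by a randomly rotated mesh, with a Scene component tracking stack height.
; Ingredient types and patty doneness are recorded, with doneness also driving the patty material.
; The top bun completes the burger and enables grabbing; dropping sphere-traces and messages the hit actor.
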(event OnDropped(GrabComponent)
  (CallFunction|PlateTrace))

(event Collision|EventHit
  (params (MyComp :type Primitive%20Component%20Object%20Reference) (Other :type Actor%20Object%20Reference) (OtherComp :type Primitive%20Component%20Object%20Reference) (bSelfMoved :type Boolean) (HitLocation :type Vector :default "0, 0, 0") (HitNormal :type Vector :default "0, 0, 0") (NormalImpulse :type Vector :default "0, 0, 0") (Hit :type Hit%20Result%20Structure%20%28by%20ref%29))
  (if (== Other "/Game/KofteciYunus/Blueprints/Ingredients/BP_Ingredient.BP_Ingredient")
    (CallFunction|AddIngredient Other)))

(fn ConstructionScript
  (|CallParentFunction))

(fn AddIngredient
  (params (Ingredient :type Actor%20Object%20Reference))
  (if (not (Variables|Default|GetCompleated))
    (bind (_offset _ingredients _pattydegree) (Class|BPIInterract|AddBurgerIngredient(Message) Ingredient self))
    (if (Utilities|Enum|NotEqual(Enum) "NewEnumerator5" _ingredients)
      (Actor|DestroyActor Ingredient)
      (Variables|Default|SetLastOffset _offset)
      (bind _returnvalue (AddComponent|AddStaticMeshComponent false (Math|Transform|MakeTransform (+ (/ _offset 2.0) (/ (Variables|Default|GetLastOffset) 2.0) (Variables|/Script/Engine.SceneComponent|GetRelativeLocation (Variables|Default|GetScene))) (Math|Rotator|MakeRotator 0.0 0.0 (Math|Random|RandomFloatinRange 0.0 3.6e+02)) "1.000000,1.000000,1.000000")))
      (Collision|SetCollisionEnabled _returnvalue "QueryOnly")
      (Transformation|SetRelativeLocation (Variables|Default|GetScene) (+ (/ _offset 2.0) (/ (Variables|Default|GetLastOffset) 2.0) (Variables|/Script/Engine.SceneComponent|GetRelativeLocation (Variables|Default|GetScene))) false false)
      (Components|StaticMesh|SetStaticMesh _returnvalue (Utilities|Select :Index _ingredients :NewEnumerator0 "/Game/KofteciYunus/Assets/StaticMeshes/SM_Patty.SM_Patty" :NewEnumerator1 "/Game/KofteciYunus/Assets/StaticMeshes/SM_Lettuce.SM_Lettuce" :NewEnumerator2 "/Game/KofteciYunus/Assets/StaticMeshes/SM_TomatoSlice.SM_TomatoSlice" :NewEnumerator3 "/Game/KofteciYunus/Assets/StaticMeshes/SM_Cheese.SM_Cheese" :NewEnumerator4 "/Game/KofteciYunus/Assets/StaticMeshes/SM_TopBun.SM_TopBun" :NewEnumerator5 "/Engine/EditorMeshes/ArcadeEditorSphere.ArcadeEditorSphere"))
      (Transformation|AttachComponentToComponent _returnvalue (Variables|Default|GetCylinder) "None" "KeepRelative" "KeepRelative" "KeepRelative" true)
      (Utilities|Array|Add (Variables|Default|GetIngredients) _ingredients)
      (switch Utilities|FlowControl|Switch|SwitchonE_Ingredient _ingredients
        (:NewEnumerator0
          (bind _returnvalue_2 (Rendering|Material|CreateDynamicMaterialInstance _returnvalue 0 (Rendering|Material|GetMaterial _returnvalue 0) "None" :!class /Script/Engine.PrimitiveComponent))
          (Utilities|Array|Add (Variables|Default|GetPatty%20Degrees) _pattydegree)
          (Rendering|Material|SetScalarParameterValue _returnvalue_2 "Cook_Factor" _pattydegree :!class /Script/Engine.MaterialInstanceDynamic))
        (:NewEnumerator4
          (Variables|Default|SetCompleated true)
          (Variables|/Game/KofteciYunus/Blueprints/Player/GrabComponent.GrabComponent_C|SetCanBeGrabbed (Variables|Default|GetGrabComponent) true)
          (Physics|SetEnableGravity (Variables|Default|GetCylinder) false))))))

(fn AddBurgerIngredient
  (params (Base :type BP%20Bread%20Base%20Object%20Reference))
  (return "0, 0, 0" "NewEnumerator5" 0.0))

(fn PlateTrace
  (bind _cylinder (Variables|Default|GetCylinder))
  (bind _returnvalue (Transformation|GetWorldLocation _cylinder))
  (bind _outhit (Collision|SphereTraceByChannel _returnvalue _returnvalue 1e+01 "TraceTypeQuery1" false 0 "None"))
  (Class|BPIInterract|SendBurgertoPlate(Message) (.HitActor (Collision|BreakHitResult _outhit)) (Variables|Default|GetIngredients) (Variables|Default|GetPatty%20Degrees) self))