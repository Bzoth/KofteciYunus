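; BP_Lettuce is a grabbable lettuce ingredient that can go into a burger or a salad.
; When dropped, a small sphere trace at its cylinder sends the salad-ingredient message to the actor it hits.
; When added to a burger, it stores the base bun and returns its height offset and ingredient type.
; Once it has a bun, it forwards anything that hits it to that bun as the next ingredient.
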(event OnDropped(GrabComponent)
  (bind _cylinder (Variables|Default|GetCylinder))
  (bind _returnvalue (Transformation|GetWorldLocation _cylinder))
  (bind _outhit (Collision|SphereTraceByChannel _returnvalue _returnvalue 1e+01 "TraceTypeQuery1" false 0 "None"))
  (Class|BPIInterract|AddSaladIngredient(Message) (.HitActor (Collision|BreakHitResult _outhit)) "NewEnumerator0" self))

(event Collision|EventHit
  (params (MyComp :type Primitive%20Component%20Object%20Reference) (Other :type Actor%20Object%20Reference) (OtherComp :type Primitive%20Component%20Object%20Reference) (bSelfMoved :type Boolean) (HitLocation :type Vector :default "0, 0, 0") (HitNormal :type Vector :default "0, 0, 0") (NormalImpulse :type Vector :default "0, 0, 0") (Hit :type Hit%20Result%20Structure%20%28by%20ref%29))
  (bind _basebun (Variables|Default|GetBaseBun)
    (:then
      (Default|AddIngredient _basebun Other))
    (:else)))

(fn ConstructionScript
  (|CallParentFunction))

(fn AddBurgerIngredient
  (params (Base :type BP%20Bread%20Base%20Object%20Reference))
  (Variables|Default|SetBaseBun Base)
  (return (Variables|Default|GetHeightOffset) "NewEnumerator1" 0.0))