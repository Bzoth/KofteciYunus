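; BP_IngredientSpawner is an ingredient dispenser that spawns an actor of its Ingredient class at its own transform when play begins.
; SpawnIngridient tracks the newest actor as LastIngredient, unbinding the previous one's Grabbed event and binding the new one's.
; This moving Grabbed binding suggests a refill each time the current ingredient is taken, though the bound handler is not shown.
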(event EventBeginPlay
  (CallFunction|SpawnIngridient))

(fn ConstructionScript)

(fn SpawnIngridient
  (bind _returnvalue (Game|SpawnActorfromClass (Variables|Default|GetIngredient) (Transformation|GetActorTransform) "Undefined" "MultiplyWithRoot" 0 0))
  (Utilities|IsValid (Variables|Default|GetLastIngredient)
    (:Is%20Valid
      (EventDispatchers|UnbindEventfromGrabbed (Variables|Default|GetLastIngredient) (EventDispatchers|CreateEvent :!event SpawnIngridient)))
    (:Is%20Not%20Valid
      _))
  (bind _output_get (Variables|Default|SetLastIngredient _returnvalue))
  (EventDispatchers|BindEventtoGrabbed _output_get (EventDispatchers|CreateEvent :!event SpawnIngridient)))