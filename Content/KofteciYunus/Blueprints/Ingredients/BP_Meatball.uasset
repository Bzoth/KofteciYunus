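; BP_Meatball is a cookable patty ingredient that stacks onto a burger bun.
; A looping timer raises the dynamic material's Cook_Factor, feeds a camera-facing WBP_CookBar, and makes the patty grabbable once cooked.
; Grabbing or StopCooking ends the timer and hides the bar; a Burn function exists but is not called here.
; Offset stores the bun and returns stack height and doneness, and Hit forwards touching actors to that bun.
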(event OnGrabbed(GrabComponent)
  (CallFunction|EndCookingTimer))

(event Custom|CookingTimer
  (CallFunction|SetWidgetLookatPlayer)
  (switch Utilities|FlowControl|Switch|SwitchonE_CookingState (Variables|Default|GetCookingState)
    (:NewEnumerator0
      (CallFunction|Cook (Variables|Default|GetCookTime)))
    (:NewEnumerator1
      (Utilities|Time|ClearandInvalidateTimerbyHandle (Variables|Default|GetCookTİmerHandler)))))

(event EventStopCooking
  (CallFunction|EndCookingTimer))

(event Collision|EventHit
  (params (MyComp :type Primitive%20Component%20Object%20Reference) (Other :type Actor%20Object%20Reference) (OtherComp :type Primitive%20Component%20Object%20Reference) (bSelfMoved :type Boolean) (HitLocation :type Vector :default "0, 0, 0") (HitNormal :type Vector :default "0, 0, 0") (NormalImpulse :type Vector :default "0, 0, 0") (Hit :type Hit%20Result%20Structure%20%28by%20ref%29))
  (bind _basebun (Variables|Default|GetBaseBun)
    (:then
      (Default|AddIngredient _basebun Other))
    (:else)))

(event EventBeginPlay
  (bind _cylinder (Variables|Default|GetCylinder))
  (bind _returnvalue (Rendering|Material|CreateDynamicMaterialInstance _cylinder 0 (Rendering|Material|GetMaterial _cylinder 0) "None" :!class /Script/Engine.PrimitiveComponent))
  (Variables|Default|SetDynamic%20Material _returnvalue)
  (bind _aswbp_cook_bar (Utilities|Casting|CastToWBP_CookBar (UserInterface|GetWidget (Variables|Default|GetWidget))))
  (Default|AssignDelagates _aswbp_cook_bar self))

(event EventStartCooking
  (bind _returnvalue (Utilities|Time|SetTimerbyEvent (delegate Custom|CookingTimer) 0.1 true))
  (Variables|Default|SetCookTİmerHandler _returnvalue)
  (CallFunction|SetBarVisible)
  (Physics|SetEnableGravity (Variables|Default|GetCylinder) true))

(fn ConstructionScript
  (|CallParentFunction))

(fn Cook
  (params (CookTime :type Float%20%28double-precision%29))
  (bind _dynamic_material (Variables|Default|GetDynamic%20Material))
  (bind _returnvalue (Rendering|Material|GetScalarParameterValue _dynamic_material "Cook_Factor" :!class /Script/Engine.MaterialInstanceDynamic))
  (Default|CallSetProgressBarValue (+ _returnvalue (/ 1.0 (* CookTime 1e+01))))
  (if (<= (+ _returnvalue (/ 1.0 (* CookTime 1e+01))) 1.0)
    (Rendering|Material|SetScalarParameterValue _dynamic_material "Cook_Factor" (+ _returnvalue (/ 1.0 (* CookTime 1e+01))) :!class /Script/Engine.MaterialInstanceDynamic)
    (return false)
    (else
      (Rendering|Material|SetScalarParameterValue _dynamic_material "Cook_Factor" 1.0 :!class /Script/Engine.MaterialInstanceDynamic)
      (Variables|Default|SetCookingState "NewEnumerator1")
      (Variables|/Game/KofteciYunus/Blueprints/Player/GrabComponent.GrabComponent_C|SetCanBeGrabbed (Variables|Default|GetGrabComponent) true)
      (return true))))

(fn Burn
  (params (Burn%20Tİme :type Float%20%28double-precision%29))
  (bind _dynamic_material (Variables|Default|GetDynamic%20Material))
  (bind _returnvalue (Rendering|Material|GetScalarParameterValue _dynamic_material "Burnt" :!class /Script/Engine.MaterialInstanceDynamic))
  (Default|CallSetProgressBarValue (+ _returnvalue (/ 1.0 (* Burn%20Tİme 1e+01))))
  (if (<= (+ _returnvalue (/ 1.0 (* Burn%20Tİme 1e+01))) 1.0)
    (Rendering|Material|SetScalarParameterValue _dynamic_material "Burnt" (+ _returnvalue (/ 1.0 (* Burn%20Tİme 1e+01))) :!class /Script/Engine.MaterialInstanceDynamic)
    (return false)
    (else
      (Rendering|Material|SetScalarParameterValue _dynamic_material "Burnt" 1.0 :!class /Script/Engine.MaterialInstanceDynamic)
      (Variables|Default|SetCookingState "NewEnumerator2")
      (return true))))

(fn Offset
  (params (Base :type BP%20Bread%20Base%20Object%20Reference))
  (Variables|Default|SetBaseBun Base)
  (bind _returnvalue (Rendering|Material|GetScalarParameterValue (Variables|Default|GetDynamic%20Material) "Cook_Factor" :!class /Script/Engine.MaterialInstanceDynamic))
  (return "0.000000,0.000000,4.100000" "NewEnumerator0" _returnvalue))

(fn SetBarVisible
  (Rendering|SetVisibility (Variables|Default|GetWidget) true false)
  (Transformation|SetWorldLocation (Variables|Default|GetWidget) (+ (Transformation|GetActorLocation) "0.000000,0.000000,10.000000") false false))

(fn SetWidgetLookatPlayer
  (Transformation|SetWorldRotation (Variables|Default|GetWidget) (Math|Rotator|FindLookatRotation (Transformation|GetWorldLocation (Variables|Default|GetWidget)) (Camera|GetCameraLocation (Game|GetPlayerCameraManager 0))) false false))

(fn EndCookingTimer
  (Rendering|SetVisibility (Variables|Default|GetWidget) false false)
  (Utilities|Time|ClearandInvalidateTimerbyHandle (Variables|Default|GetCookTİmerHandler))
  (Physics|SetEnableGravity (Variables|Default|GetCylinder) false)
  (Utilities|FlowControl|DoOnce false
    (:Completed
      (Default|CallGrabbed))))