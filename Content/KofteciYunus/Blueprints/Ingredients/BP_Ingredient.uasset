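; Base ingredient actor for food assembly that can be grabbed, dropped and stacked onto a bread base.
; The first grab fires CallGrabbed, and a drop enables physics and runs a small sphere trace that passes the ingredient to any BP_BreadBase hit.
; A dropped bread base, itself a child class, only gets physics once completed.
; The Offset function returns default stacking offset, ingredient type and patty degree.
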(event OnGrabbed(GrabComponent)
  (Utilities|FlowControl|DoOnce false
    (:Completed
      (Default|CallGrabbed))))

(event OnDropped(GrabComponent)
  (bind _cylinder (Variables|Default|GetCylinder))
  (bind _returnvalue (Transformation|GetWorldLocation _cylinder))
  (if (!= (Utilities|GetClass self) "/Game/KofteciYunus/Blueprints/Ingredients/BP_BreadBase.BP_BreadBase_C")
    (Physics|SetSimulatePhysics (Variables|Default|GetCylinder) true)
    (bind _outhit (Collision|SphereTraceByChannel _returnvalue _returnvalue 1e+01 "TraceTypeQuery1" false 0 "None"))
    (if (== "/Game/KofteciYunus/Blueprints/Ingredients/BP_BreadBase.BP_BreadBase_C" (Utilities|GetClass (.HitActor (Collision|BreakHitResult _outhit))))
      (bind _asbp_bread_base (Utilities|Casting|CastToBP_BreadBase (.HitActor (Collision|BreakHitResult _outhit))))
      (Default|AddIngredient _asbp_bread_base self))
    (else
      (bind _asbp_bread_base_2 (Utilities|Casting|CastToBP_BreadBase self))
      (if (Variables|/Game/KofteciYunus/Blueprints/Ingredients/BP_BreadBase.BP_BreadBase_C|GetCompleated _asbp_bread_base_2)
        (Physics|SetSimulatePhysics (Variables|Default|GetCylinder) true)))))

(fn ConstructionScript)

(fn Offset
  (params (Base :type BP%20Bread%20Base%20Object%20Reference))
  (return "0.000000,0.000000,2.000000" "NewEnumerator5" 0.0))